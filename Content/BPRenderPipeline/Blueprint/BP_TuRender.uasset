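; Hand-built render pipeline Blueprint that rasterizes the Cube mesh into the RT_Depth render target once at BeginPlay.
; It reads triangles through a procedural mesh copy and projects vertices with WordToScreen, a manual perspective projection using Tcamera and FOV.
; Each triangle feeds screen UVs, mesh UVs and inverse depths to M_DrawDepth and is drawn as a canvas triangle.
; After each triangle, M_CopyRT is drawn into RT_DepthTemp.
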(event EventBeginPlay
  (Rendering|ClearRenderTarget2D "/Game/BPRenderPipeline/RenderTarget/RT_Depth.RT_Depth")
  (Class|KismetProceduralMeshLibrary|CopyProceduralMeshfromStaticMeshComponent (Variables|Default|GetCube) 0 (Variables|Default|GetProceduralMesh) false)
  (Variables|Default|SetT (Transformation|GetRelativeTransform (Variables|Default|GetCube)))
  (bind _returnvalue (Rendering|Material|CreateDynamicMaterialInstance "/Game/BPRenderPipeline/Mats/M_DrawDepth.M_DrawDepth" "None" "None" :!class /Script/Engine.KismetMaterialLibrary))
  (Variables|Default|SetDepthPainter _returnvalue)
  (bind (_vertices _triangles _normals _uvs) (Class|KismetProceduralMeshLibrary|GetSectionfromProceduralMesh (Variables|Default|GetProceduralMesh)))
  (for _index (range 0 (- (/ (Utilities|Array|Length _triangles) 3) 1))
    (Variables|Default|SetAindex (Utilities|Array|Get(acopy) _triangles (+ (* _index 3) 0)))
    (Variables|Default|SetBindex (Utilities|Array|Get(acopy) _triangles (+ (* _index 3) 1)))
    (Variables|Default|SetCindex (Utilities|Array|Get(acopy) _triangles (+ (* _index 3) 2)))
    (bind (_canvas _size _context) (Rendering|BeginDrawCanvastoRenderTarget "/Game/BPRenderPipeline/RenderTarget/RT_Depth.RT_Depth"))
    (Variables|Default|SetSize _size)
    (Rendering|Material|SetVectorParameterValue (Variables|Default|GetDepthPainter) "PointA" (CallFunction|ToDepthParam (.ScreenUV (CallFunction|WordtoScreen (Math|Transform|TransformLocation (Variables|Default|GetT) (Utilities|Array|Get(acopy) _vertices (Variables|Default|GetAindex))))) (Utilities|Array|Get(acopy) _uvs (Variables|Default|GetAindex))) :!class /Script/Engine.MaterialInstanceDynamic)
    (Rendering|Material|SetVectorParameterValue (Variables|Default|GetDepthPainter) "PointB" (CallFunction|ToDepthParam (.ScreenUV (CallFunction|WordtoScreen (Math|Transform|TransformLocation (Variables|Default|GetT) (Utilities|Array|Get(acopy) _vertices (Variables|Default|GetBindex))))) (Utilities|Array|Get(acopy) _uvs (Variables|Default|GetBindex))) :!class /Script/Engine.MaterialInstanceDynamic)
    (Rendering|Material|SetVectorParameterValue (Variables|Default|GetDepthPainter) "PointC" (CallFunction|ToDepthParam (.ScreenUV (CallFunction|WordtoScreen (Math|Transform|TransformLocation (Variables|Default|GetT) (Utilities|Array|Get(acopy) _vertices (Variables|Default|GetCindex))))) (Utilities|Array|Get(acopy) _uvs (Variables|Default|GetCindex))) :!class /Script/Engine.MaterialInstanceDynamic)
    (Rendering|Material|SetVectorParameterValue (Variables|Default|GetDepthPainter) "InvDepth" (Utilities|Struct|MakeLinearColor (/ 1.0 (.Z (CallFunction|WordtoScreen (Math|Transform|TransformLocation (Variables|Default|GetT) (Utilities|Array|Get(acopy) _vertices (Variables|Default|GetAindex)))))) (/ 1.0 (.Z (CallFunction|WordtoScreen (Math|Transform|TransformLocation (Variables|Default|GetT) (Utilities|Array|Get(acopy) _vertices (Variables|Default|GetBindex)))))) (/ 1.0 (.Z (CallFunction|WordtoScreen (Math|Transform|TransformLocation (Variables|Default|GetT) (Utilities|Array|Get(acopy) _vertices (Variables|Default|GetCindex)))))) 0.0) :!class /Script/Engine.MaterialInstanceDynamic)
    (Class|Canvas|DrawMaterialTriangle _canvas (Variables|Default|GetDepthPainter) (Utilities|Array|MakeArray (Utilities|Struct|MakeCanvasUVTri (* (Variables|Default|GetSize) (.ScreenUV (CallFunction|WordtoScreen (Math|Transform|TransformLocation (Variables|Default|GetT) (Utilities|Array|Get(acopy) _vertices (Variables|Default|GetAindex)))))) (.ScreenUV (CallFunction|WordtoScreen (Math|Transform|TransformLocation (Variables|Default|GetT) (Utilities|Array|Get(acopy) _vertices (Variables|Default|GetAindex))))) "(R=1.000000,G=1.000000,B=1.000000,A=1.000000)" (* (Variables|Default|GetSize) (.ScreenUV (CallFunction|WordtoScreen (Math|Transform|TransformLocation (Variables|Default|GetT) (Utilities|Array|Get(acopy) _vertices (Variables|Default|GetBindex)))))) (.ScreenUV (CallFunction|WordtoScreen (Math|Transform|TransformLocation (Variables|Default|GetT) (Utilities|Array|Get(acopy) _vertices (Variables|Default|GetBindex))))) "(R=1.000000,G=1.000000,B=1.000000,A=1.000000)" (* (Variables|Default|GetSize) (.ScreenUV (CallFunction|WordtoScreen (Math|Transform|TransformLocation (Variables|Default|GetT) (Utilities|Array|Get(acopy) _vertices (Variables|Default|GetCindex)))))) (.ScreenUV (CallFunction|WordtoScreen (Math|Transform|TransformLocation (Variables|Default|GetT) (Utilities|Array|Get(acopy) _vertices (Variables|Default|GetCindex))))) "(R=1.000000,G=1.000000,B=1.000000,A=1.000000)")))
    (Rendering|EndDrawCanvastoRenderTarget _context)
    (Rendering|DrawMaterialtoRenderTarget "/Game/BPRenderPipeline/RenderTarget/RT_DepthTemp.RT_DepthTemp" "/Game/BPRenderPipeline/Mats/M_CopyRT.M_CopyRT")))

(fn ConstructionScript)

(fn WordtoScreen
  (params (Location :type Vector))
  (bind _size (Variables|Default|GetSize))
  (bind _tcamera (Variables|Default|GetTcamera))
  (bind _returnvalue (Math|Transform|InverseTransformLocation _tcamera Location))
  (bind (_x _y _z) (Math|Vector|BreakVector _returnvalue))
  (return (+ (* (/ (Math|Vector2D|MakeVector2D _y _z) (* _x (* (Math|Vector2D|MakeVector2D 1.0 (/ (.y _size) (.x _size))) (Math|Trig|Tan(Degrees) (/ (Variables|Default|GetFOV) 2.0))))) "(X=0.500000,Y=-0.500000)") "(X=0.500000,Y=0.500000)") _x))

(fn ToDepthParam
  (params (Position :type Vector%202D%20Structure) (MeshUV :type Vector%202D%20Structure))
  (bind (_x _y) (Math|Vector2D|BreakVector2D Position))
  (bind (_x_2 _y_2) (Math|Vector2D|BreakVector2D MeshUV))
  (return (Utilities|Struct|MakeLinearColor _x _y _x_2 _y_2)))