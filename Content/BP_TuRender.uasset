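; BP_TuRender is an unfinished experiment that appears aimed at rasterizing mesh triangles into a depth render target.
; On BeginPlay it copies the Cube static mesh into a ProceduralMesh, reads section 0 and walks its index buffer one triangle at a time.
; The loop only extracts vertex indices.
; Camera-space vertex transforms, mesh section creation and canvas triangle drawing to RT_Depth are present but unconnected, so nothing is rendered.
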(event EventBeginPlay
  (bind _proceduralmesh (Variables|Default|GetProceduralMesh))
  (bind _cube (Variables|Default|GetCube))
  (Class|KismetProceduralMeshLibrary|CopyProceduralMeshfromStaticMeshComponent _cube 0 _proceduralmesh false)
  (Variables|Default|SetT (Transformation|GetRelativeTransform _cube))
  (bind (_vertices _triangles) (Class|KismetProceduralMeshLibrary|GetSectionfromProceduralMesh _proceduralmesh))
  (for _index (range 0 (- (/ (Utilities|Array|Length _triangles) 3) 1))
    (Variables|Default|SetAindex (Utilities|Array|Get(acopy) _triangles (+ (* _index 3) 0)))
    (Variables|Default|SetBindex (Utilities|Array|Get(acopy) _triangles (+ (* _index 3) 1)))
    (Variables|Default|SetCindex (Utilities|Array|Get(acopy) _triangles (+ (* _index 3) 2)))))

(fn ConstructionScript)